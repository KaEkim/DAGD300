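; SpikeWallBP is a spike wall actor that moves vertically between its starting position and a point 400 units above it.
; BeginPlay stores the start location, and Tick drives the movement from the IsMurder flag.
; While IsMurder is true, Delay nodes in Tick and a Switch toggle snap the wall up and down every half second.
; Otherwise, Tick holds it at the raised position.
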(event `self.ReceiveBeginPlay`
  (bind _output_get (set `self.OriginalPos` (`self.K2_GetActorLocation`))))

(event `self.ReceiveTick`
  (params (DeltaSeconds :type "Float (single-precision)"))
  (if (`self.isMurder`)
    (if (`self.switch`)
      (`KismetSystemLibrary.Delay` 0.5)
      (set `self.switch` false)
      (`self.K2_SetActorRelativeLocation` (stale `self.ReceiveBeginPlay` _output_get))
      (else
        (`KismetSystemLibrary.Delay` 0.5)
        (set `self.switch` true)
        (`self.K2_SetActorRelativeLocation` (+ (stale `self.ReceiveBeginPlay` _output_get) (0.0 0.0 400.0)) :!label _label)))
    (else
      (goto _label))))

(fn `UserConstructionScript`)