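; BoosBP is an actor in the town map, apparently a boss, that periodically spawns batches of BoosBP1 actors around itself while facing the player.
; A frame-counted cooldown on Tick triggers each batch, placing spawns at randomized multiples of Offset in local space, lowered toward the ground.
; Tick also turns its yaw toward the player through MoveComponentTo.
; Once Iisded is true, it stops both behaviors and destroys itself after a delay.
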(event `self.ReceiveBeginPlay`
  (set `self.coolDown` 0))

(event `self.ReceiveTick`
  (params (DeltaSeconds :type "Float (single-precision)"))
  (if (`self.iisded`)
    (`KismetSystemLibrary.Delay` 5.0)
    (`self.K2_DestroyActor`)
    (else
      (set `self.coolDown` (- (`self.coolDown`) 1))
      (if true
        (`|ExecutionSequence`
          (:`then_0`
            ;[1 1 1] StillNeedCooldown
            (if (<= (`self.coolDown`) 0)
              (set `self.coolDown` 150)
              ;[1 1 1] Repeat x Times
              (set `self.Counter` 0)
              (while (<= (`self.Counter`) 10)
                ;[1 1 1] Spawn
                (`|SpawnActorFromClass` "/Game/Town_Map/BoosBP1.BoosBP1_C" (`KismetMathLibrary.Conv_VectorToTransform` (`KismetMathLibrary.MakeVector` (.x (`KismetMathLibrary.TransformLocation` (`self.GetTransform`) (+ (* (`self.Offset`) (`KismetMathLibrary.RandomInteger` 40)) (0.0 0.0 -25.0)))) (.y (`KismetMathLibrary.TransformLocation` (`self.GetTransform`) (+ (* (`self.Offset`) (`KismetMathLibrary.RandomInteger` 40)) (0.0 0.0 -25.0)))) (- (.z (`KismetMathLibrary.TransformLocation` (`self.GetTransform`) (+ (* (`self.Offset`) (`KismetMathLibrary.RandomInteger` 40)) (0.0 0.0 -25.0)))) 60.0))) "AdjustIfPossibleButAlwaysSpawn" "OverrideRootScale" null null)
                ;[1 1 1] Increment
                (set `self.Counter` (+ (`self.Counter`) 1)))))
          (:`then_1`
            (`KismetSystemLibrary.MoveComponentTo` (`self.RootComponent`) (`self.K2_GetActorLocation`) (`KismetMathLibrary.MakeRotator` (.roll (`self.K2_GetActorRotation`)) (.pitch (`self.K2_GetActorRotation`)) (.yaw (`KismetMathLibrary.FindLookAtRotation` (`self.K2_GetActorLocation`) (`self.K2_GetActorLocation` (`GameplayStatics.GetPlayerPawn` 0))))))))))))

(fn `UserConstructionScript`)